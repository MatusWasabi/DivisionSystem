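; Functional test that checks the division presenter's level getter stays stable across repeated calls, guarding against a pure function that mutates Blueprint state.
; PrepareTest creates a division view widget, spawns BP_DivisionPresenter with that view and a Model, then sets the given experience points.
; StartTest calls GetCurrentLevel in a configurable loop, printing each result, then passes or fails on one final comparison with the expected level.
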(event EventPrepareTest
  (bind _returnvalue (UserInterface|CreateWidget "/DivisionSystem/Core/WBP_DivisionView.WBP_DivisionView_C"))
  (bind _returnvalue_2 (Game|SpawnActorfromClass "/DivisionSystem/Core/BP_DivisionPresenter.BP_DivisionPresenter_C" (Math|Transform|MakeTransform "0, 0, 0" "0, 0, 0" "1.000000,1.000000,1.000000") "Undefined" "MultiplyWithRoot" 0 _returnvalue (Variables|Default|GetModel) 0))
  (bind _output_get (Variables|Default|SetPresenter _returnvalue_2))
  (Default|SetExperiencePoint _output_get (Variables|Default|GetGivenPoint)))

(event EventStartTest
  (bind _presenter (Variables|Default|GetPresenter))
  (bind _level (Default|GetCurrentLevel _presenter))
  ;[1 1 1] Preventing Calling Pure function that will mutate blueprint states
  (for _index (range 0 (Math|Conversions|ToInteger(Byte) (Variables|Default|GetNumberCallingTime)))
    (Development|PrintString (Utilities|String|ToString(Text) (Utilities|Text|FormatText "At {time} Level is {level}" _index _level))))
  (bind _returnvalue (Class|FunctionalTest|AssertEqualInt (Math|Conversions|ToInteger(Byte) _level) (Math|Conversions|ToInteger(Byte) (Variables|Default|GetExpectedLevel))))
  (if _returnvalue
    (Class|FunctionalTest|FinishTest "Succeeded")
    (else
      (Class|FunctionalTest|FinishTest "Failed"))))

(fn ConstructionScript)