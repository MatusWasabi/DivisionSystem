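; BP_GetNextTitle is a functional test that checks the title a division presenter reports as next for a given level.
; PrepareTest creates a WBP_DivisionView widget, spawns a BP_DivisionPresenter wired to it and the test's Model, then applies GivenLevel.
; StartTest compares GetNextTitle against Expected as a Name and finishes as succeeded or failed.
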(event EventPrepareTest
  (bind _returnvalue (UserInterface|CreateWidget "/DivisionSystem/Core/WBP_DivisionView.WBP_DivisionView_C"))
  (bind _returnvalue_2 (Game|SpawnActorfromClass "/DivisionSystem/Core/BP_DivisionPresenter.BP_DivisionPresenter_C" (Math|Transform|MakeTransform "0, 0, 0" "0, 0, 0" "1.000000,1.000000,1.000000") "Undefined" "MultiplyWithRoot" 0 _returnvalue (Variables|Default|GetModel) 0))
  (bind _output_get (Variables|Default|SetPresenter _returnvalue_2))
  (Default|SetLevel _output_get (Variables|Default|GetGiven%20Level)))

(event EventStartTest
  (bind _returnvalue (Class|FunctionalTest|AssertEqualName (Default|GetNextTitle (Variables|Default|GetPresenter)) (Variables|Default|GetExpected)))
  (if _returnvalue
    (Class|FunctionalTest|FinishTest "Succeeded")
    (else
      (Class|FunctionalTest|FinishTest "Failed"))))

(fn ConstructionScript)