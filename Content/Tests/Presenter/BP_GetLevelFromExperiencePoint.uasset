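; Functional test that checks the division presenter derives the expected career level from a given amount of experience points.
; PrepareTest creates a division view widget, spawns BP_DivisionPresenter with that view and a model, then sets the career experience.
; StartTest compares the presenter's career level with the expected one and finishes as succeeded or failed.
; It then loads the FTEST_GetTitleFromLevel level instance, apparently chaining to the next test.
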(event EventPrepareTest
  (bind _returnvalue (UserInterface|CreateWidget "/DivisionSystem/Core/WBP_DivisionView.WBP_DivisionView_C"))
  (bind _returnvalue_2 (Game|SpawnActorfromClass "/DivisionSystem/Core/BP_DivisionPresenter.BP_DivisionPresenter_C" (Math|Transform|MakeTransform "0, 0, 0" "0, 0, 0" "1.000000,1.000000,1.000000") "Undefined" "MultiplyWithRoot" 0 _returnvalue (Variables|Default|GetModel) 0))
  (bind _output_get (Variables|Default|SetPresenter _returnvalue_2))
  (Default|SetCareerExperiencePoint _output_get (Variables|Default|GetExperienceGiven)))

(event EventStartTest
  (bind _levelexpected (Variables|Default|GetLevelExpected))
  (bind _returnvalue (Math|Conversions|ToInteger(Byte) _levelexpected))
  (bind _returnvalue_2 (Class|FunctionalTest|AssertEqualInt (Math|Conversions|ToInteger(Byte) (Default|GetCareerLevel (Variables|Default|GetPresenter))) _returnvalue))
  (if _returnvalue_2
    (Class|FunctionalTest|FinishTest "Succeeded" (Utilities|String|ToString(Text) (Utilities|Text|FormatText "The level is {lvel}" _returnvalue)))
    (else
      (Class|FunctionalTest|FinishTest "Failed" (Utilities|String|ToString(Text) (Utilities|Text|FormatText "Sry, but the level is {level}" 0)))))
  (Class|LevelStreamingDynamic|LoadLevelInstancebySoftObjectPtr "/DivisionSystem/Tests/Presenter/FTEST_GetTitleFromLevel.FTEST_GetTitleFromLevel" "0, 0, 0" "0, 0, 0" "" 0 false))

(fn ConstructionScript)