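; Functional test that checks the title a division presenter returns for a given level.
; On prepare, it creates a WBP_DivisionView widget, spawns BP_DivisionPresenter with that view and the DA_ModelSample model, then sets the configured level.
; On start, it compares the presenter's title with the expected name and finishes as succeeded or failed.
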(event EventPrepareTest
  (bind _returnvalue (UserInterface|CreateWidget "/DivisionSystem/Core/WBP_DivisionView.WBP_DivisionView_C"))
  (bind _returnvalue_2 (Game|SpawnActorfromClass "/DivisionSystem/Core/BP_DivisionPresenter.BP_DivisionPresenter_C" (Math|Transform|MakeTransform "0, 0, 0" "0, 0, 0" "1.000000,1.000000,1.000000") "Undefined" "MultiplyWithRoot" 0 _returnvalue "/DivisionSystem/Sample/DA_ModelSample.DA_ModelSample" 0))
  (bind _output_get (Variables|Default|SetPresenter _returnvalue_2))
  (Default|SetLevel _output_get (Variables|Default|GetGivenLevel)))

(event EventStartTest
  (bind _expectedtitle (Variables|Default|GetExpectedTitle))
  (bind _returnvalue (Class|FunctionalTest|AssertEqualName (Default|GetTitle (Variables|Default|GetPresenter)) _expectedtitle (Utilities|String|ToString(Text) (Utilities|Text|FormatText "The actual title is {title}. The expected {expected}" 0 _expectedtitle))))
  (if _returnvalue
    (Class|FunctionalTest|FinishTest "Succeeded")
    (else
      (Class|FunctionalTest|FinishTest "Failed"))))

(fn ConstructionScript)