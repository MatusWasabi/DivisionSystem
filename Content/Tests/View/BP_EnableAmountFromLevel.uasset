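; BP_EnableAmountFromLevel is a functional test that checks how many nodes WBP_DivisionView enables for a given level.
; PrepareTest creates the widget, adds it to the viewport and sets its displayed node count.
; StartTest calls EnableSubNodes with the level and edge parameters, then passes or fails by comparing the enabled node count to the expected value.
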(event EventPrepareTest
  (bind _returnvalue (UserInterface|CreateWidget "/DivisionSystem/Core/WBP_DivisionView.WBP_DivisionView_C"))
  (bind _output_get (Variables|Default|SetView _returnvalue))
  (UserInterface|Viewport|AddtoViewport _output_get 0)
  (Variables|/DivisionSystem/Core/WBP_DivisionView.WBP_DivisionView_C|SetNumber%20Of%20Display%20Node (Variables|Default|GetView) (Variables|Default|GetNumber%20Of%20Display%20Node)))

(event EventStartTest
  (bind _view (Variables|Default|GetView))
  (Default|EnableSubNodes _view (Variables|Default|GetGivenLevel) (Variables|Default|GetBegin%20Edge) (Variables|Default|GetEdge%20Difference))
  (bind _returnvalue (Class|FunctionalTest|AssertEqualInt (Default|GetNumberOfEnabledNodes _view) (Math|Conversions|ToInteger(Byte) (Variables|Default|GetExpectedNumberOfNodeEnable))))
  (if _returnvalue
    (Class|FunctionalTest|FinishTest "Succeeded")
    (else
      (Class|FunctionalTest|FinishTest "Failed"))))

(fn ConstructionScript)