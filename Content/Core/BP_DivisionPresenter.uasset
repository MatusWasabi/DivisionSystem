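; BP_DivisionPresenter is the presenter between a division Model and View, showing career level progress within the current division.
; Setting the career base level or experience points refreshes the View.
; The Model converts both values into a current level, then supplies that division's edges plus icons and titles for the current and next division.
; The View receives these to enable progress sub-nodes and update both border icons and titles.
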(fn ConstructionScript)

(fn GetTitle
  (bind _model (Variables|Default|GetModel))
  (bind _output_get (Variables|Default|SetTitle (Default|GetTitlefromLevel _model (Default|GetLevelfromExperiencePoint _model (Variables|Default|GetExperiencePoint) (Variables|Default|GetBaseLevel)))))
  (return _output_get))

(fn SetLevel
  (params (CareerLevel :type Byte))
  (Variables|Default|SetBaseLevel CareerLevel)
  (CallFunction|UpdateView))

(fn GetCurrentLevel
  (return (Default|GetLevelfromExperiencePoint (Variables|Default|GetModel) (Variables|Default|GetExperiencePoint) (Variables|Default|GetBaseLevel))))

(fn GetCurrentIcon
  (bind _model (Variables|Default|GetModel))
  (bind _output_get (Variables|Default|SetCurrentIcon (Default|GetIconfromLevel _model (Default|GetLevelfromExperiencePoint _model (Variables|Default|GetExperiencePoint) (Variables|Default|GetBaseLevel)))))
  (return _output_get))

(fn GetNextIcon
  (bind _output_get (Variables|Default|SetNextIcon (Default|GetIconfromLevel (Variables|Default|GetModel) (Default|GetEndEdgeOfLevel (Variables|Default|GetModel) (Default|GetLevelfromExperiencePoint (Variables|Default|GetModel) (Variables|Default|GetExperiencePoint) (Variables|Default|GetBaseLevel))))))
  (return _output_get))

(fn GetEdgesDifference
  (bind _output_get (Variables|Default|SetEdgeDifference (Default|GetEdgesDifference (Variables|Default|GetModel) (Default|GetLevelfromExperiencePoint (Variables|Default|GetModel) (Variables|Default|GetExperiencePoint) (Variables|Default|GetBaseLevel)))))
  (return _output_get))

(fn GetNextTitle
  (bind _output_get (Variables|Default|SetNextTitle (Default|GetTitlefromLevel (Variables|Default|GetModel) (Default|GetEndEdgeOfLevel (Variables|Default|GetModel) (Default|GetLevelfromExperiencePoint (Variables|Default|GetModel) (Variables|Default|GetExperiencePoint) (Variables|Default|GetBaseLevel))))))
  (return _output_get))

(fn GetBeginEdge
  (return (Default|GetBeginEdgeOfLevel (Variables|Default|GetModel) (ConfigurationMediator|GetCurrentLevel))))

(fn SetExperiencePoint
  (params (ExperiencePoint :type Integer))
  (Variables|Default|SetExperiencePoint ExperiencePoint)
  (CallFunction|UpdateView))

(fn UpdateView
  (Default|EnableSubNodes (Variables|Default|GetView) (ConfigurationMediator|GetCurrentLevel) (ConfigurationMediator|GetBeginEdge) (ConfigurationMediator|GetEdgesDifference))
  (Default|UpdateBordersIcon (Variables|Default|GetView) (ConfigurationMediator|GetCurrentIcon) (CallFunction|GetNextIcon))
  (Default|UpdateBordersText (Variables|Default|GetView) (ConfigurationMediator|GetTitle) (CallFunction|GetNextTitle)))