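; Division progression model that maps player levels to experience requirements, titles and icons through threshold-keyed maps.
; Lookups scan keys for the bracket containing a level; several stop at the first higher key, so they assume ascending order.
; XP-to-level conversion repeatedly subtracts each level's requirement, then clamps to MaximumLevel as a byte.
; Level-to-XP conversion reverses this by summing requirement times levels spanned in each bracket.
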(fn GetExperiencePointRequired
  (params (CurrentLevel :type Byte))
  (bind _keys (Utilities|Map|Keys (Variables|Default|GetLevelExperienceRequired)))
  (bind _array_element (Utilities|Array|ForEachLoopwithBreak _keys :!label _label)
    (:LoopBody
      ;[1 1 1] Keep finding level req. Not using early return as early return method will break if collections is not ordered in order.
      (if (>= CurrentLevel _array_element)
        (LocalVariables|Setexperience (.Value (Utilities|Map|Find (Variables|Default|GetLevelExperienceRequired) _array_element)))
        (else
          (goto _label Break))))
    (:Completed
      (return (LocalVariables|Getexperience)))))

(fn GetTitlefromLevel
  (params (Level :type Byte))
  (bind _keys (Utilities|Map|Keys (Variables|Default|GetLevelTitles)))
  ;[1 1 1] Find the higher level till the end. Why not early return? Ans: That will need data asset to be in order
  (for _array_element _keys
    (if (>= Level _array_element)
      (LocalVariables|SetReturn%20Title (.Value (Utilities|Map|Find (Variables|Default|GetLevelTitles) _array_element)))))
  (return (LocalVariables|GetReturn%20Title)))

(fn GetIconfromLevel
  (params (Level :type Byte))
  (bind _keys (Utilities|Map|Keys (Variables|Default|GetLevelIcons)))
  ;[1 1 1] Keep track of lower key to that texture. Not using early return as early return method will break if collections is not ordered in order.
  (for _array_element _keys
    (if (>= Level _array_element)
      (LocalVariables|SetTextureKey _array_element)))
  (return (.Value (Utilities|Map|Find (Variables|Default|GetLevelIcons) (LocalVariables|GetTextureKey)))))

(fn GetBeginEdgeOfLevel
  (params (Level :type Byte))
  (bind _keys (Utilities|Map|Keys (Variables|Default|GetLevelExperienceRequired)))
  ;[1 1 1] Keep track of lower edge. Not using early return as early return method will break if collections is not ordered in order.
  (for _array_element _keys
    (if (>= Level _array_element)
      (LocalVariables|SetEdge _array_element)))
  (return (LocalVariables|GetEdge)))

(fn GetEdgesDifference
  (params (Level :type Byte))
  (bind _keys (Utilities|Map|Keys (Variables|Default|GetLevelExperienceRequired)))
  ;[1 1 1] Keep track of begin and end edge. Not using early return as early return method will break if collections is not ordered in order.
  (bind _array_element (Utilities|Array|ForEachLoopwithBreak _keys :!label _label)
    (:LoopBody
      (if (>= Level _array_element)
        (LocalVariables|SetBeginEdge _array_element)
        (else
          (LocalVariables|SetEndEdge _array_element)
          (goto _label Break))))
    (:Completed
      (return (- (LocalVariables|GetEndEdge) (LocalVariables|GetBeginEdge))))))

(fn GetLevelfromExperiencePoint
  (params (ExperiencePoint :type Integer) (BaseLevel :type Byte :default 1))
  (bind _output_get (LocalVariables|SetCurrentLevel BaseLevel))
  ;[1 1 1] Keep track of total experience point
  (bind _output_get_2 (LocalVariables|SetLeftoverExperiencePoint ExperiencePoint))
  (while (>= _output_get_2 (CallFunction|GetExperiencePointRequired _output_get))
    (LocalVariables|SetLeftoverExperiencePoint (- (LocalVariables|GetLeftoverExperiencePoint) (CallFunction|GetExperiencePointRequired (LocalVariables|GetCurrentLevel))))
    ;[1 1 1] Keep tracking of level that required point will based on
    (LocalVariables|SetCurrentLevel (+ (LocalVariables|GetCurrentLevel) 1)))
  (return (Math|Conversions|ToByte(Integer) (Math|Integer|Clamp(Integer) (Math|Conversions|ToInteger(Byte) (LocalVariables|GetCurrentLevel)) 0 (Math|Conversions|ToInteger(Byte) (Variables|Default|GetMaximumLevel))))))

(fn GetEndEdgeOfLevel
  (params (Level :type Byte))
  (bind _keys (Utilities|Map|Keys (Variables|Default|GetLevelExperienceRequired)))
  ;[1 1 1] Finding what is bigger than given level. The bigger one of keys is the end edge or upper edge.
  (for _array_element _keys
    (if (< Level _array_element)
      (return _array_element)))
  (bind _keys_2 (Utilities|Map|Keys (Variables|Default|GetLevelExperienceRequired)))
  (return (Utilities|Array|Get(acopy) _keys_2 (Utilities|Array|LastIndex _keys_2))))

(fn GetExperiencePointfromLevel
  (params (Level :type Byte :default 1))
  (bind _keys (Utilities|Map|Keys (Variables|Default|GetLevelExperienceRequired)))
  (for _array_element _keys
    ;[1 1 1] Reversing Get Level From Experience Point
    (if (> Level _array_element)
      (LocalVariables|SetExperienceReturn (+ (LocalVariables|GetExperienceReturn) (* (CallFunction|GetExperiencePointRequired _array_element) (Math|Integer|Clamp(Integer) (- Level _array_element) 0 (Math|Conversions|ToInteger(Byte) (Edges|GetEdgesDifference _array_element))))))))
  (return (LocalVariables|GetExperienceReturn)))